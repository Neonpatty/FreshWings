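; Player character Blueprint, despite the PlayerController name, that handles mouse look, movement, jumping, sprinting and shooting.
; Tick polls the look axes, whose names appear swapped: Up_Down drives yaw and inverted Left_Right drives pitch.
; Movement axes push along actor forward and right vectors, and jumping requires being on the ground.
; Shoot spawns a Bullet at the Muzzle, while Sprint toggles max walk speed, both with debug prints.
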(event `self.ReceiveTick`
  (params (DeltaSeconds :type "Float (single-precision)"))
  ;[0 0.3326 1] Mouse Look
  (`self.AddControllerYawInput` (`self.GetInputAxisValue`))
  (`self.AddControllerPitchInput` (* (`self.GetInputAxisValue`) -1.0)))

(event `InputAxis|Move_Forward_Back`
  (params (AxisValue :type "Float (single-precision)"))
  ;[0 0.3326 1] Movement
  ;;[0.8744 0 1] Move Forward and Backwards
  (`self.AddMovementInput` (`self.GetActorForwardVector`) AxisValue))

(event `InputAction|Jump`
  (params (Key :type "Key Structure"))
  ;[0 0.3326 1] Jumping
  (:`Pressed`
    (if (`NavMovementComponent.IsMovingOnGround` (`self.CharacterMovement`))
      (`self.Jump`))))

(event `InputAxis|Move_Left_Right`
  (params (AxisValue :type "Float (single-precision)"))
  ;[0 0.3326 1] Movement
  ;;[0.8744 0 1] Move Left and right
  (`self.AddMovementInput` (`self.GetActorRightVector`) AxisValue))

(event `InputAction|Shoot`
  (params (Key :type "Key Structure"))
  ;[0 0.3326 1] Shooting
  (:`Pressed`
    (`KismetSystemLibrary.PrintString` "FIRED")
    (`|SpawnActorFromClass` "/Game/Blueprints/Bullet.Bullet_C" (`SceneComponent.K2_GetComponentToWorld` (`self.Muzzle`)) "Undefined" "OverrideRootScale" null null)))

(event `InputAction|Sprint`
  (params (Key :type "Key Structure"))
  (bind _charactermovement (`self.CharacterMovement`))
  ;[0 0.3326 1] Sprint
  (:`Pressed`
    (`KismetSystemLibrary.PrintString` "Sprinting")
    (set `CharacterMovementComponent.MaxWalkSpeed` (`self.Sprint Speed`) _charactermovement))
  (:`Released`
    (`KismetSystemLibrary.PrintString` "Walking")
    (set `CharacterMovementComponent.MaxWalkSpeed` (`self.Walk Speed`) _charactermovement)))

(fn `UserConstructionScript`)