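; Bullet is a projectile actor moved by a ProjectileMovement component, with a Sphere component for hit detection.
; On BeginPlay it copies its InitialSpeed and ProjectileGravityScale variables into the movement component.
; The first Sphere hit, gated by DoOnce, destroys the bullet and prints the name of the actor it hit, with no damage applied.
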(event `self.ReceiveBeginPlay`
  (bind _projectilemovement (`self.ProjectileMovement`))
  ;[0 0.3326 1] Sets Bullet Speed and Bullet Gravity
  (`|ExecutionSequence`
    (:`then_0`
      (set `ProjectileMovementComponent.InitialSpeed` (`self.Initial Speed`) _projectilemovement))
    (:`then_1`
      (set `ProjectileMovementComponent.ProjectileGravityScale` (`self.Projectile Gravity Scale`) _projectilemovement))))

(event `self.Sphere.OnComponentHit`
  (params (HitComponent :type "PrimitiveComponent Object Reference") (OtherActor :type "Actor Object Reference") (OtherComp :type "PrimitiveComponent Object Reference") (NormalImpulse :type "Vector Structure") (Hit :type "HitResult Structure (by ref)"))
  ;[0 0.3326 1] Destroys bullet when hits an actor
  (`|ExecutionSequence`
    (:`then_1`
      (`/Engine/EditorBlueprintResources/StandardMacros.DoOnce` false
        (:`Completed`
          (`|ExecutionSequence`
            (:`then_0`
              (`self.K2_DestroyActor`))
            (:`then_1`
              (`KismetSystemLibrary.PrintString` (`KismetSystemLibrary.GetObjectName` OtherActor)))))))))

(fn `UserConstructionScript`)