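; Target actor that takes a random point value on spawn and is destroyed when shot by a Bullet.
; A hit on its Cube component that casts to Bullet prints the value, then destroys the actor after a configurable delay.
; The value is only printed, and the game mode's RespawnTarget call is disconnected, so the Destroyed event does nothing.
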(event `self.ReceiveBeginPlay`
  ;[0 0.3326 1] Sets Target Vaule on Spawn
  (set `self.TargetValue` (`KismetMathLibrary.RandomIntegerInRange` 10 250)))

(event `self.Cube.OnComponentHit`
  (params (HitComponent :type "PrimitiveComponent Object Reference") (OtherActor :type "Actor Object Reference") (OtherComp :type "PrimitiveComponent Object Reference") (NormalImpulse :type "Vector Structure") (Hit :type "HitResult Structure (by ref)"))
  ;[0 0.3326 1] When Target is hit by a bullet, Give Points and Destory Target
  (cast `/Game/Blueprints/Bullet` OtherActor)
  (`|ExecutionSequence`
    (:`then_1`
      (`KismetSystemLibrary.PrintString` (`KismetStringLibrary.Conv_IntToString` (`self.TargetValue`))))
    (:`then_2`
      (`KismetSystemLibrary.Delay` (`self.DelayToDestroy`))
      (`self.K2_DestroyActor`))))

(event `self.ReceiveDestroyed`
  ;[0 0.3326 1] When Target is Destroyed, Spawn a new one
)

(fn `UserConstructionScript`)